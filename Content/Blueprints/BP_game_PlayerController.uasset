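; Player controller Blueprint that puts the in-game UI on screen for the local player.
; BeginPlay creates a BP_UI_InGame widget, stores it as GameUI and adds it to the viewport.
; Tick is empty; disconnected leftover logic would show CurrentFPS in the widget, red below 58 and green otherwise, despite a note saying 30.
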(event EventBeginPlay
  ;[1 1 1] Display UI
  (if (Pawn|IsLocalPlayerController)
    (bind _returnvalue (UserInterface|CreateWidget "/Game/Visuals/Widgets/BP_UI_InGame.BP_UI_InGame_C"))
    (bind _output_get (Variables|Default|SetGame_UI _returnvalue))
    (UserInterface|Viewport|AddtoViewport _output_get 0)))

(event EventTick
  (params (DeltaSeconds :type Float%20%28single-precision%29)))

(fn ConstructionScript)